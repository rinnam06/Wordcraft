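; BP_Exit is an interactable exit that returns the player to the street map.
; Overlapping its box shows interact text and enables input only if the game instance's IsWorked flag is set.
; Leaving the box hides the text and disables input.
; Pressing E sets the game instance's StreetPoint, likely the arrival spot, and opens street_Map.
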(event `self.InteractBox.OnComponentBeginOverlap`
  (params (OverlappedComponent :type "PrimitiveComponent Object Reference") (OtherActor :type "Actor Object Reference") (OtherComp :type "PrimitiveComponent Object Reference") (OtherBodyIndex :type Integer) (bFromSweep :type Boolean) (SweepResult :type "HitResult Structure (by ref)"))
  (bind _returnvalue (`GameplayStatics.GetPlayerCharacter` 0))
  (if (== OtherActor _returnvalue)
    (cast `/Game/FirstPerson/Blueprints/BP_FirstPersonCharacter` _returnvalue)
    (bind _asgi_my_game (cast `/Game/_Wordcraft/GI_MyGame` (`GameplayStatics.GetGameInstance`)))
    (`SceneComponent.SetVisibility` (`self.InteractText`) true false)
    (if (`/Game/_Wordcraft/GI_MyGame.IsWorked?` _asgi_my_game)
      (`self.EnableInput` (`GameplayStatics.GetPlayerController` 0))
      (else
        (`self.DisableInput` (`GameplayStatics.GetPlayerController` 0))))))

(event `self.InteractBox.OnComponentEndOverlap`
  (params (OverlappedComponent :type "PrimitiveComponent Object Reference") (OtherActor :type "Actor Object Reference") (OtherComp :type "PrimitiveComponent Object Reference") (OtherBodyIndex :type Integer))
  (bind _returnvalue (`GameplayStatics.GetPlayerCharacter` 0))
  (if (== OtherActor _returnvalue)
    (cast `/Game/FirstPerson/Blueprints/BP_FirstPersonCharacter` _returnvalue)
    (`SceneComponent.SetVisibility` (`self.InteractText`) false false)
    (`self.DisableInput` (`GameplayStatics.GetPlayerController` 0))))

(event `Key|E`
  (params (Key :type "Key Structure"))
  (:`Pressed`
    (bind _asgi_my_game (cast `/Game/_Wordcraft/GI_MyGame` (`GameplayStatics.GetGameInstance`)))
    (set `/Game/_Wordcraft/GI_MyGame.StreetPoint` 4 _asgi_my_game)
    (`GameplayStatics.OpenLevel` "street_Map")))

(fn `UserConstructionScript`)