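; BP_TutorialDrop is a drop zone for the placement tutorial that accepts tutorial items whose target zone matches its own.
; On box overlap, if the player is not holding anything, it checks the overlapping item's zone name against ExpectedZoneName.
; A match destroys the item after a short delay and increments the player character's Score; a mismatch prints a retry message.
; A Score of four flags placement as finished on GI_MyGame and calls TutorialFinish.
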(event `self.Box.OnComponentBeginOverlap`
  (params (OverlappedComponent :type "PrimitiveComponent Object Reference") (OtherActor :type "Actor Object Reference") (OtherComp :type "PrimitiveComponent Object Reference") (OtherBodyIndex :type Integer) (bFromSweep :type Boolean) (SweepResult :type "HitResult Structure (by ref)"))
  (bind _asbp_first_person_character (cast `/Game/FirstPerson/Blueprints/BP_FirstPersonCharacter` (`GameplayStatics.GetPlayerCharacter` 0)))
  (if (not (`/Game/FirstPerson/Blueprints/BP_FirstPersonCharacter.IsHolding?` _asbp_first_person_character))
    (`self.CheckAnswer` OtherActor)))

(event `CheckAnswer`
  (params (ItemToCheck :type "Actor Object Reference"))
  (bind _asbp_tutorial_item (cast `/Game/_Wordcraft/_Blueprint/BP_TutorialItem` ItemToCheck))
  (if (`KismetStringLibrary.EqualEqual_StrStr` (`/Game/_Wordcraft/_Blueprint/BP_TutorialItem.MyTargetZone` _asbp_tutorial_item) (`self.ExpectedZoneName`))
    (`KismetSystemLibrary.Delay` 0.2)
    (`self.K2_DestroyActor` _asbp_tutorial_item)
    (bind _asbp_first_person_character (cast `/Game/FirstPerson/Blueprints/BP_FirstPersonCharacter` (`GameplayStatics.GetPlayerCharacter` 0)))
    (bind _result (`/Engine/EditorBlueprintResources/StandardMacros.IncrementInt` (`/Game/FirstPerson/Blueprints/BP_FirstPersonCharacter.Score` _asbp_first_person_character))
      (:`  `
        (bind _output_get (set `/Game/FirstPerson/Blueprints/BP_FirstPersonCharacter.Score` _result _asbp_first_person_character))
        (if (== _output_get 4)
          (bind _asgi_my_game (cast `/Game/_Wordcraft/GI_MyGame` (`GameplayStatics.GetGameInstance`)))
          (set `/Game/_Wordcraft/GI_MyGame.PlaceTutorialFinish` true _asgi_my_game)
          (`/Game/_Wordcraft/GI_MyGame.TutorialFinish` _asgi_my_game)
          (`KismetSystemLibrary.PrintString` "Tutorial Place Completed"))))
    (else
      (`KismetSystemLibrary.PrintString` "Wrong! Try again." true true (struct :`G` 0.66 :`B` 1.0 :`A` 1.0) 5.0))))

(fn `UserConstructionScript`)