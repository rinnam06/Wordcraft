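; BP_DropZone is a drop zone that scores items placed in the correct zone.
; On box overlap, if the first-person player is not holding anything, it checks whether the BP_TestItem's MyTargetZone matches its ExpectedZoneName.
; A match destroys the item after a short delay and increments the player character's Score, calling WinPlaceRoom once the score reaches the hard-coded target.
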(event `self.Box.OnComponentBeginOverlap`
  (params (OverlappedComponent :type "PrimitiveComponent Object Reference") (OtherActor :type "Actor Object Reference") (OtherComp :type "PrimitiveComponent Object Reference") (OtherBodyIndex :type Integer) (bFromSweep :type Boolean) (SweepResult :type "HitResult Structure (by ref)"))
  (bind _asbp_first_person_character (cast `/Game/FirstPerson/Blueprints/BP_FirstPersonCharacter` (`GameplayStatics.GetPlayerCharacter` 0)))
  (if (not (`/Game/FirstPerson/Blueprints/BP_FirstPersonCharacter.IsHolding?` _asbp_first_person_character))
    (`self.CheckAnswer` OtherActor)))

(event `CheckAnswer`
  (params (ItemToCheck :type "Actor Object Reference"))
  (bind _asbp_test_item (cast `/Game/_Wordcraft/_Blueprint/BP_TestItem` ItemToCheck))
  (if (`KismetStringLibrary.EqualEqual_StrStr` (`/Game/_Wordcraft/_Blueprint/BP_TestItem.MyTargetZone` _asbp_test_item) (`self.ExpectedZoneName`))
    (`KismetSystemLibrary.Delay` 0.2)
    (`self.K2_DestroyActor` _asbp_test_item)
    (bind _asbp_first_person_character (cast `/Game/FirstPerson/Blueprints/BP_FirstPersonCharacter` (`GameplayStatics.GetPlayerCharacter` 0)))
    (bind _result (`/Engine/EditorBlueprintResources/StandardMacros.IncrementInt` (`/Game/FirstPerson/Blueprints/BP_FirstPersonCharacter.Score` _asbp_first_person_character))
      (:`  `
        (bind _output_get (set `/Game/FirstPerson/Blueprints/BP_FirstPersonCharacter.Score` _result _asbp_first_person_character))
        (if (>= _output_get 20)
          (`/Game/FirstPerson/Blueprints/BP_FirstPersonCharacter.WinPlaceRoom` _asbp_first_person_character))))))

(fn `UserConstructionScript`)