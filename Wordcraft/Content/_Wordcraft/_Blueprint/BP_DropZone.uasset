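; BP_DropZone is a sorting target that checks whether a BP_TestItem dropped into it belongs there.
; On box overlap it compares the item's MyTargetZone to its own ExpectedZoneName.
; A match adds a point to Score on the player's BP_FirstPersonCharacter, destroys the item after a short delay and prints the score.
; A mismatch only prints a retry message and leaves the item in place.
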(event `self.Box.OnComponentBeginOverlap`
  (params (OverlappedComponent :type "PrimitiveComponent Object Reference") (OtherActor :type "Actor Object Reference") (OtherComp :type "PrimitiveComponent Object Reference") (OtherBodyIndex :type Integer) (bFromSweep :type Boolean) (SweepResult :type "HitResult Structure (by ref)"))
  (bind _asbp_test_item (cast `/Game/_Wordcraft/_Blueprint/BP_TestItem` OtherActor))
  (if (`KismetStringLibrary.EqualEqual_StrStr` (`/Game/_Wordcraft/_Blueprint/BP_TestItem.MyTargetZone` _asbp_test_item) (`self.ExpectedZoneName`))
    (bind _asbp_first_person_character (cast `/Game/FirstPerson/Blueprints/BP_FirstPersonCharacter` (`GameplayStatics.GetPlayerCharacter` 0)))
    (bind _output_get (set `/Game/FirstPerson/Blueprints/BP_FirstPersonCharacter.Score` (+ (`/Game/FirstPerson/Blueprints/BP_FirstPersonCharacter.Score` _asbp_first_person_character) 1) _asbp_first_person_character))
    (`KismetSystemLibrary.Delay` 0.2)
    (`self.K2_DestroyActor` _asbp_test_item)
    (`KismetSystemLibrary.PrintString` "Correct!!!")
    (`KismetSystemLibrary.PrintString` (`KismetStringLibrary.Conv_IntToString` _output_get))
    (else
      (`KismetSystemLibrary.PrintString` "Wrong! Try again." true true (struct :`G` 0.66 :`B` 1.0 :`A` 1.0) 5.0))))

(fn `UserConstructionScript`)