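; BP_Exit is a double-door exit that swings open and shut.
; It exposes OpenDoor and CloseDoor events, with no trigger logic of its own.
; Each event plays a separate timeline per leaf from the start, driving the yaw of Hinge and Hinge2.
; Opening and closing use different timelines, so each motion always restarts from the beginning of its curve instead of reversing.
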(event `CloseDoor`
  (`|ExecutionSequence`
    (:`then_0`
      (bind (_direction _closedoor) (`Timeline|LeftDoorAnimation` :!via `PlayFromStart`)
        (:`Update`
          (`SceneComponent.K2_SetRelativeRotation` (`self.Hinge`) (`KismetMathLibrary.MakeRotator` 0.0 0.0 _closedoor) false false))))
    (:`then_1`
      (bind (_direction_2 _closedoor_2) (`Timeline|RightDoorAnimation` :!via `PlayFromStart`)
        (:`Update`
          (`SceneComponent.K2_SetRelativeRotation` (`self.Hinge2`) (`KismetMathLibrary.MakeRotator` 0.0 0.0 _closedoor_2) false false))))))

(event `OpenDoor`
  (`|ExecutionSequence`
    (:`then_0`
      (bind (_direction _closedoor _opendoor) (`Timeline|Timeline_1` :!via `PlayFromStart`)
        (:`Update`
          (`SceneComponent.K2_SetRelativeRotation` (`self.Hinge`) (`KismetMathLibrary.MakeRotator` 0.0 0.0 _opendoor) false false))))
    (:`then_1`
      (bind (_direction_2 _closedoor_2 _opendoor_2) (`Timeline|Timeline_0` :!via `PlayFromStart`)
        (:`Update`
          (`SceneComponent.K2_SetRelativeRotation` (`self.Hinge2`) (`KismetMathLibrary.MakeRotator` 0.0 0.0 _opendoor_2) false false))))))

(fn `UserConstructionScript`)