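; Test item actor that randomizes its mesh and a "put the item in a place" quest on BeginPlay.
; It picks a random ItemPool entry and a random MyQuests_Place data table row, then builds MyQuestText from both and stores the row's zone as MyTargetZone.
; Highlighting toggles the mesh's custom depth stencil value, and OnInteract only prints a debug string.
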(event `self.ReceiveBeginPlay`
  (bind _itempool (`self.ItemPool`))
  (bind (_output_itemname _output_itemmesh) (break `/Game/_Wordcraft/ST_ItemPlace` (`|GetArrayItem` _itempool (`self.LockedRandomIndex`))))
  (bind _outrownames (`DataTableFunctionLibrary.GetDataTableRowNames` "/Game/_Wordcraft/MyQuests_Place.MyQuests_Place"))
  (set `self.LockedRandomIndex` (`KismetMathLibrary.RandomIntegerInRange` 0 (`KismetArrayLibrary.Array_LastIndex` _itempool)))
  (bind _returnvalue (`|GetDataTableRow` "/Game/_Wordcraft/MyQuests_Place.MyQuests_Place" (`|GetArrayItem` _outrownames (`KismetMathLibrary.RandomIntegerInRange` 0 (`KismetArrayLibrary.Array_LastIndex` _outrownames))))
    (:`then`
      (set `self.MyQuestText` (`KismetTextLibrary.Conv_StringToText` (`KismetStringLibrary.Concat_StrStr` "Put the " (`KismetTextLibrary.Conv_TextToString` _output_itemname) " " (`KismetTextLibrary.Conv_TextToString` (break `/Game/_Wordcraft/ST_QuestPlace` _returnvalue)))))
      (set `self.MyTargetZone` (`.ZoneString_5_D7BDAF9945B2F306AE5144A554FF74FF` (break `/Game/_Wordcraft/ST_QuestPlace` _returnvalue)))
      (`StaticMeshComponent.SetStaticMesh` (`self.StaticMesh`) _output_itemmesh))))

(event `/Game/_Wordcraft/BPI_Interact.OnInteract`
  (`KismetSystemLibrary.PrintString` "Pick me!"))

(event `EnableHighlight`
  (`PrimitiveComponent.SetCustomDepthStencilValue` (`self.StaticMesh`) 1))

(event `DisableHighlight`
  (`PrimitiveComponent.SetCustomDepthStencilValue` (`self.StaticMesh`) 0))

(fn `UserConstructionScript`)